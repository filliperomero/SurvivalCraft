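; BP_WoodCeiling is a wooden ceiling piece in the survival-crafting building system.
; On BeginPlay it passes its twelve snap boxes to SetSnapBoxes in a single array, four each for ceilings, walls and triangle ceilings.
; The graph holds no other logic, and the construction script is empty.
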(event `self.ReceiveBeginPlay`
  (`self.SetSnapBoxes` (`|MakeArray` (`self.CeilingBox`) (`self.CeilingBox1`) (`self.CeilingBox2`) (`self.CeilingBox3`) (`self.WallBox`) (`self.WallBox1`) (`self.WallBox2`) (`self.WallBox3`) (`self.TriangleCeilingBox`) (`self.TriangleCeilingBox1`) (`self.TriangleCeilingBox3`) (`self.TriangleCeilingBox2`))))

(fn `UserConstructionScript`)