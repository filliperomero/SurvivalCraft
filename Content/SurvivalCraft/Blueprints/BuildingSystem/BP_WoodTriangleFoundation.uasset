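; BP_WoodTriangleFoundation is a wooden triangle foundation piece in the SurvivalCraft building system.
; On BeginPlay it passes its snap box components to SetSnapBoxes.
; The boxes come in three groups of three, named for square foundation, triangle foundation and wall attachments.
; The construction script is empty.
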(event `self.ReceiveBeginPlay`
  (`self.SetSnapBoxes` (`|MakeArray` (`self.FoundationBox`) (`self.FoundationBox1`) (`self.FoundationBox2`) (`self.TriangleFoundationBox`) (`self.TriangleFoundationBox1`) (`self.TriangleFoundationBox2`) (`self.WallBox`) (`self.WallBox1`) (`self.WallBox2`))))

(fn `UserConstructionScript`)